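; Rat character Blueprint with self-contained wandering AI that idles, roams, eats and flees, driving Rat_AnimBlueprint action states.
; Delay-based event loops and boolean guards pick behavior from random rolls and a hunger meter that drains, then refills while eating.
; AI Perception startles it into running to random reachable points around its start location.
; Hits drain health to death; a delayed Alive restores health, but its state reset is disconnected.
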(event OnTargetPerceptionUpdated(AIPerception)
  (params (Actor :type Actor%20Object%20Reference) (Stimulus :type AI%20Stimulus%20Structure))
  ;[1 1 1] Detect
  (|CheckSeenDeadRun
    (:else
      (Variables|Booleans|SetSeen? true)
      (Components|Movement|StopMovementImmediately (Variables|Character|GetCharacterMovement))
      (bind _asrat_anim_blueprint (Utilities|Casting|CastToRat_AnimBlueprint (|GetAnim4)))
      (Variables|/Game/Medhue_Rat/Blueprints/Rat_AnimBlueprint.Rat_AnimBlueprint_C|SetRat_Actions _asrat_anim_blueprint "NewEnumerator5")
      (|DetectResetBooleans)
      (Utilities|FlowControl|Delay 0.8)
      (CallFunction|RunAway)
      (Utilities|FlowControl|Delay 4.0)
      (Variables|Booleans|SetSeen? false))))

(event Custom|Decide%20Action
  (params (Skip%20Delay? :type Boolean))
  ;[1 1 1] Decide
  (if Skip%20Delay?
    (|CheckDeadWaitRestingEatingHungryTired_2 :!label _label
      (:No%20Timer
        (if (not (Variables|Booleans|GetDead?)) :!label _label_2
          (if (Variables|Booleans|GetHungry?)
            (Utilities|FlowControl|Delay 1.0 :!label _label_3)
            (CallFunction|Eating)
            (elif (<= (Variables|IntegersUsed|GetDecide%20Logic) 3)
              (Utilities|FlowControl|Delay 1.0)
              (CallFunction|Roam)
              (CallFunction|DrainHunger)
              (else
                (Variables|Booleans|SetHungry? true :!label _label_4)
                (goto _label_3))))
          (CallFunction|RandomLogic)))
      (:Idle%20Timer
        (if (< (Variables|Default|GetHealth) 100)
          (CallFunction|RegainHealth))
        (Variables|IntegersUsed|SetDecide%20Logic (Math|Random|RandomIntegerinRange 1 4))
        (Variables|IntegersUsed|SetIdle%20Random%20Count 0)
        (Variables|IntegersUsed|SetIdle%20Random%20Time (Math|Random|RandomIntegerinRange (Variables|Default|GetIdle%20Time%20Min) (Variables|Default|GetIdle%20Time%20Max)))
        (Variables|Booleans|SetWait? true)
        (|IdleTimeLoop_2 :!label _label_5
          (:Time%20Up
            (goto _label_2))
          (:Hungry
            (Variables|IntegersUsed|SetDecide%20Logic 4)
            (goto _label_4))
          (:Loop%20Out
            (Utilities|FlowControl|Delay 1.0)
            (goto _label_5 Loop%20In)))))
    (else
      (goto _label execute2))))

(event Custom|Random%20Logic
  ;[1 1 1] Logic
  (Utilities|FlowControl|Delay 2.0)
  (Variables|Booleans|SetLogic? true)
  (Variables|IntegersUsed|SetDecide%20Logic%20Time 0)
  (if (<= (Variables|IntegersUsed|GetDecide%20Logic) 3)
    _
    (else
      (if (Variables|Booleans|GetEating?) :!label _label
        (Variables|IntegersUsed|SetDecide%20Logic%20Random (Math|Random|RandomIntegerinRange (Variables|Default|GetEating%20Time%20Min) (Variables|Default|GetEating%20Time%20Max)))
        (Variables|IntegersUsed|SetDecide%20Logic%20Time 0)
        (Utilities|FlowControl|Delay 1.0 :!label _label_2)
        (bind _output_get (Variables|IntegersUsed|SetDecide%20Logic%20Time (+ (Variables|IntegersUsed|GetDecide%20Logic%20Time) 1)))
        (if (== _output_get (Variables|IntegersUsed|GetDecide%20Logic%20Random))
          (Variables|IntegersUsed|SetDecide%20Logic (Math|Random|RandomIntegerinRange 1 4))
          (goto _label)
          (elif (Variables|Booleans|GetEating?)
            (if (Variables|Booleans|GetRun?)
              _
              (else
                (goto _label_2)))))
        (else
          (Variables|Booleans|SetHungry? false)))))
  (Variables|Booleans|SetLogic? false))

(event Custom|Run%20Away
  ;[1 1 1] Run Away
  (if (not (Variables|Booleans|GetDead?))
    (Variables|/Script/Engine.CharacterMovementComponent|SetMaxWalkSpeed (Variables|Character|GetCharacterMovement) (Variables|Default|GetRun%20Speed))
    (bind _asrat_anim_blueprint (Utilities|Casting|CastToRat_AnimBlueprint (|GetAnim1)))
    (Variables|/Game/Medhue_Rat/Blueprints/Rat_AnimBlueprint.Rat_AnimBlueprint_C|SetRat_Actions _asrat_anim_blueprint "NewEnumerator0")
    (Variables|Booleans|SetWait? true)
    (AI|AIMoveTo self (|GetRandomRunPointinRange (Variables|Default|GetRun%20Radius%20Min) (Variables|Default|GetRun%20Radius%20Max)) 0 5.0 false
      (:OnSuccess
        (|RunResetBooleans2)
        (CallFunction|Roam))
      (:OnFail
        (|RunResetBooleans1)
        (CallFunction|DecideAction true)))))

(event Custom|Eating
  ;[1 1 1] Eat
  (|CheckDeadRun
    (:else
      (Components|Movement|StopMovementImmediately (Variables|Character|GetCharacterMovement))
      (bind _asrat_anim_blueprint (Utilities|Casting|CastToRat_AnimBlueprint (|GetAnim6)))
      (Variables|/Game/Medhue_Rat/Blueprints/Rat_AnimBlueprint.Rat_AnimBlueprint_C|SetRat_Actions _asrat_anim_blueprint "NewEnumerator1")
      (Variables|Booleans|SetEating? true)
      (CallFunction|ReGainHunger)
      (Utilities|FlowControl|Delay 1.0 :!label _label)
      (if (not (Variables|Booleans|GetDead?))
        (if (not (Variables|Booleans|GetRun?))
          (if (Variables|Booleans|GetHungry?)
            (if (>= (Variables|IntegersUsed|GetDecide%20Logic) 3)
              (goto _label)
              (else
                _)))
          (Variables|Booleans|SetEating? false)
          (Variables|Booleans|SetHungry? false)
          (Variables|/Game/Medhue_Rat/Blueprints/Rat_AnimBlueprint.Rat_AnimBlueprint_C|SetRat_Actions _asrat_anim_blueprint "NewEnumerator0")
          (Utilities|FlowControl|Delay 0.5)
          (CallFunction|DecideAction true)
          (CallFunction|DrainHunger))))))

(event Custom|Roam
  ;[1 1 1] Roam
  (|CheckRunDeadTireHungry
    (:Hungry
      _)
    (:else
      (Variables|/Script/Engine.CharacterMovementComponent|SetMaxWalkSpeed (Variables|Character|GetCharacterMovement) (Variables|Default|GetWalk%20Speed))
      (bind _asrat_anim_blueprint (Utilities|Casting|CastToRat_AnimBlueprint (|GetAnim3)))
      (Variables|/Game/Medhue_Rat/Blueprints/Rat_AnimBlueprint.Rat_AnimBlueprint_C|SetRat_Actions _asrat_anim_blueprint "NewEnumerator0")
      (Variables|Booleans|SetWait? true)
      (AI|AIMoveTo self (|GetRandomWalkPoint (Variables|Default|GetWalk%20Radius)) 0 5.0 false
        (:OnSuccess
          _)
        (:OnFail
          _))
      (Variables|Booleans|SetWait? false)))
  (CallFunction|DecideAction false))

(event Custom|Drain%20Hunger
  ;[1 1 1] Drain Hunger
  (if (not (Variables|Booleans|GetEating?))
    (if (not (Variables|Booleans|GetDead?))
      (bind _output_get (Variables|Default|SetHunger (|DrainingHunger)))
      (if (<= _output_get 1)
        (Utilities|FlowControl|Delay 1.0)
        (Variables|Booleans|SetHungry? true)
        (Variables|IntegersUsed|SetDecide%20Logic 5)
        (CallFunction|DecideAction true)
        (else
          (Utilities|FlowControl|Delay 1.0)
          (CallFunction|DrainHunger))))))

(event Custom|Re%20Gain%20Hunger
  ;[1 1 1] Regain Hunger
  (|CheckEatingDeadRun
    (:else
      (bind _output_get (Variables|Default|SetHunger (|GainingHunger)))
      (if (== _output_get (Variables|Default|GetMax%20Hunger))
        (Variables|Booleans|SetHungry? false)
        (Variables|IntegersUsed|SetDecide%20Logic 2)
        (CallFunction|DecideAction false)
        (CallFunction|DrainHunger)
        (else
          (Utilities|FlowControl|Delay 1.0)
          (CallFunction|ReGainHunger))))))

(event Custom|Regain%20Health
  ;[1 1 1] Regain Health
  (if (not (Variables|Booleans|GetDead?))
    (bind _output_get (Variables|Default|SetHealth (|GainingHealth)))
    (if (not (== _output_get (Variables|Default|GetMax%20Heath)))
      (Utilities|FlowControl|Delay 2.0)
      (CallFunction|RegainHealth))))

(event Custom|Damage
  ;[1 1 1] Damage
  (if (not (Variables|Booleans|GetDead?))
    (bind _output_get (Variables|Default|SetHealth (|DrainingHealth)))
    (if (== _output_get 0)
      (Components|Movement|StopMovementImmediately (Variables|Character|GetCharacterMovement))
      (Variables|Booleans|SetDead? true)
      (bind _asrat_anim_blueprint (Utilities|Casting|CastToRat_AnimBlueprint (|GetAnim5)))
      (Variables|/Game/Medhue_Rat/Blueprints/Rat_AnimBlueprint.Rat_AnimBlueprint_C|SetRat_Actions _asrat_anim_blueprint "NewEnumerator6")
      (Utilities|FlowControl|Delay 1.5)
      (Variables|/Game/Medhue_Rat/Blueprints/Rat_AnimBlueprint.Rat_AnimBlueprint_C|SetRat_Actions _asrat_anim_blueprint "NewEnumerator8")
      (|DamageResetBooleans2)
      (Utilities|FlowControl|Delay (|RandomDeadTimeinRange))
      (CallFunction|Alive))))

(event Custom|Alive
  ;[1 1 1] Revive
  (Variables|Default|SetHealth (Variables|Default|GetMax%20Heath)))

(event EventBeginPlay
  ;[1 1 1] Start
  (CallFunction|DecideAction false)
  (CallFunction|DrainHunger)
  (Variables|IntegersUsed|SetRat%20Location (Transformation|GetActorLocation)))

(event Collision|EventHit
  (params (MyComp :type Primitive%20Component%20Object%20Reference) (Other :type Actor%20Object%20Reference) (OtherComp :type Primitive%20Component%20Object%20Reference) (bSelfMoved :type Boolean) (HitLocation :type Vector :default "0, 0, 0") (HitNormal :type Vector :default "0, 0, 0") (NormalImpulse :type Vector :default "0, 0, 0") (Hit :type Hit%20Result%20Structure%20%28by%20ref%29))
  ;[1 1 1] Hit Check
  (if (not (Variables|Default|GetDeathOff?))
    (if (not (Variables|Booleans|GetHit?))
      (if (not (Variables|Booleans|GetDead?))
        (|HitResetBooleans)
        (CallFunction|Damage)
        (Utilities|FlowControl|Delay 5.0)
        (Variables|Booleans|SetHit? false)))))

(fn ConstructionScript)